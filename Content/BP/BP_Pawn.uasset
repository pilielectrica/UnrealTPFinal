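; BP_Pawn is a pawn that combines player-driven movement with a random NPC wander behavior.
; Possession events add and remove the IMC_Player mapping context on player controller 0, whichever controller possesses it.
; IA_Move applies a swept, fixed-step local offset built from the actor's right and forward vectors.
; BeginPlay starts a self-repeating AIMoveTo loop to random reachable nearby points, pausing after each success or failure.
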(event Custom|Move%20NPC
  (bind _output_get (Variables|Default|SetRandom%20Location (.RandomLocation (AI|Navigation|GetRandomReachablePointinRadius (Transformation|GetActorLocation) 1e+03 0 0))))
  (AI|AIMoveTo self _output_get 0 2e+01 false
    (:OnSuccess
      (Utilities|FlowControl|Delay 2.0))
    (:OnFail
      (Utilities|FlowControl|Delay 1.0)))
  (CallFunction|MoveNPC))

(event Input|EnhancedActionEvents|EnhancedInputActionIA_Move
  (params (ActionValue :type Vector%202D%20Structure) (ElapsedSeconds :type Float%20%28double-precision%29) (TriggeredSeconds :type Float%20%28double-precision%29) (InputAction :type Input%20Action%20Object%20Reference :default "/Game/ThirdPerson/Input/Actions/IA_Move.IA_Move"))
  (bind (_x _y) (Math|Vector2D|BreakVector2D ActionValue))
  (Transformation|AddActorLocalOffset (* (+ (* (Transformation|GetActorRightVector) _x) (* (Transformation|GetActorForwardVector) _y)) 1e+01) true false))

(event EventBeginPlay
  (CallFunction|MoveNPC))

(event Collision|EventActorBeginOverlap
  (params (OtherActor :type Actor%20Object%20Reference)))

(event EventTick
  (params (DeltaSeconds :type Float%20%28single-precision%29)))

(event EventPossessed
  (params (NewController :type Controller%20Object%20Reference))
  (bind _returnvalue (Game|GetPlayerController 0))
  (Utilities|IsValid _returnvalue
    (:Is%20Valid
      (Input|AddMappingContext (PlayerController|LocalPlayerSubsystems|GetEnhancedInputLocalPlayerSubsystem _returnvalue) "/Game/Input/Actions/IMC_Player.IMC_Player" 0 "(bIgnoreAllPressedKeysUntilRelease=True,bForceImmediately=False,bNotifyUserSettings=False)"))))

(event EventUnpossessed
  (params (OldController :type Controller%20Object%20Reference))
  (bind _returnvalue (Game|GetPlayerController 0))
  (Utilities|IsValid _returnvalue
    (:Is%20Valid
      (Input|RemoveMappingContext (PlayerController|LocalPlayerSubsystems|GetEnhancedInputLocalPlayerSubsystem _returnvalue) "/Game/Input/Actions/IMC_Player.IMC_Player" "(bIgnoreAllPressedKeysUntilRelease=True,bForceImmediately=False,bNotifyUserSettings=False)"))))

(fn ConstructionScript)