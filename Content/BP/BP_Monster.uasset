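; Monster Blueprint that demonstrates interactive audio driven by player distance and a keyboard-adjustable life value.
; Tick maps distance to the player onto the CB_LPF control bus through a bus mix activated on BeginPlay, giving a distance-based low-pass filter.
; E toggles the AP_Monster attack animation flag while held and, on press, plays the MetaSound and sends Vida (life) as its "vida" parameter.
; Up and Down step Vida within limits and print it.
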(event EventBeginPlay
  ;[0.15 0.15 0.15 0.5] LOW PASS FILTER LOGIC DEPENDING ON THE DISTANCE BETWEEN THE PLAYER AND THE MONSTER
  (CallFunction|ActivateBusMix)
  (CallFunction|UpdateMixbyFilter 0 "CB_LPF" 0 0 (Math|Float|MapRangeClamped (Transformation|GetDistanceTo (Game|GetPlayerCharacter 0)) 0.0 2e+03 1.0 0.0)))

(event EventTick
  (params (DeltaSeconds :type Float%20%28single-precision%29))
  ;[0.15 0.15 0.15 0.5] LOW PASS FILTER LOGIC DEPENDING ON THE DISTANCE BETWEEN THE PLAYER AND THE MONSTER
  (CallFunction|UpdateMixbyFilter 0 "CB_LPF" 0 0 (Math|Float|MapRangeClamped (Transformation|GetDistanceTo (Game|GetPlayerCharacter 0)) 0.0 2e+03 1.0 0.0)))

(event Input|KeyboardEvents|E
  (params (Key :type Key%20Structure))
  (bind _audio (Variables|Default|GetAudio))
  ;[0.15 0.15 0.15 0.5] "E" KEY PLAYS THE SOUND AND COMUNICATE OUR METASOUND WITH THE MONSTER'S LIFE VARIABLE
  (:Pressed
    (bind _asap_monster (Utilities|Casting|CastToAP_Monster (Components|SkeletalMesh|GetAnimInstance (Variables|Default|GetMonster))))
    (Variables|/Game/BP/AP_Monster.AP_Monster_C|SetIsAttacking _asap_monster true)
    (Audio|Components|Audio|Play _audio 0.0)
    (Audio|Parameter|SetFloatParameter _audio "vida" (Variables|Default|Getvida) :!class /Script/AudioExtensions.AudioParameterControllerInterface))
  (:Released
    (bind _asap_monster_2 (Utilities|Casting|CastToAP_Monster (Components|SkeletalMesh|GetAnimInstance (Variables|Default|GetMonster))))
    (bind _output_get (Variables|/Game/BP/AP_Monster.AP_Monster_C|SetIsAttacking _asap_monster_2 false))))

(event Input|KeyboardEvents|Up
  (params (Key :type Key%20Structure))
  ;[0.15 0.15 0.15 0.5] UP KEY TO INCREMENT THE MONSTER'S LIFE
  (:Pressed
    (if (< (Variables|Default|Getvida) 5.0)
      (Development|PrintString "(MONSTER'S LIFE)")
      (Variables|Default|Setvida (+ (Variables|Default|Getvida) 1.0))
      (Development|PrintString (Utilities|String|ToString(Float) (Variables|Default|Getvida))))))

(event Input|KeyboardEvents|Down
  (params (Key :type Key%20Structure))
  ;[0.15 0.15 0.15 0.5] DOWN KEY TO DECRESE THE MONSTER'S LIFE
  (:Pressed
    (if (> (Variables|Default|Getvida) 1.0)
      (Development|PrintString "(MONSTER'S LIFE) ")
      (Variables|Default|Setvida (- (Variables|Default|Getvida) 1.0))
      (Development|PrintString (Utilities|String|ToString(Float) (Variables|Default|Getvida))))))

(fn ConstructionScript)