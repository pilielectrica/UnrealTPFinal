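; Indicator light actor that turns green when the player reaches it and signals a linked trap and an optional fairy.
; The sphere material is black from construction and switches to red on BeginPlay.
; Overlap by BPC_Character_UMG turns it green and calls UnlockTrapMessage on Trampa every time.
; If a Fairy reference is valid, a DoOnce limits its FreeFairyMessage call to a single firing.
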(event EventBeginPlay
  (Rendering|Material|SetMaterial (Variables|Default|GetEsfera_Luz) 0 "/Game/Pilar_Marco/Materials/M_Color_Rojo.M_Color_Rojo"))

(event Collision|EventActorBeginOverlap
  (params (OtherActor :type Actor%20Object%20Reference))
  (bind _fairy (Variables|Default|GetFairy))
  (Utilities|Casting|CastToBPC_Character_UMG OtherActor)
  (Rendering|Material|SetMaterial (Variables|Default|GetEsfera_Luz) 0 "/Game/Pilar_Marco/Materials/M_Color_Verde.M_Color_Verde")
  (Class|BPIGame|UnlockTrap(Message) (Variables|Default|GetTrampa))
  (Utilities|IsValid _fairy
    (:Is%20Valid
      (Utilities|FlowControl|DoOnce false
        (:Completed
          (Class|BPIGame|FreeFairy(Message) _fairy))))))

(fn ConstructionScript
  (Rendering|Material|SetMaterial (Variables|Default|GetEsfera_Luz) 0 "/Game/Pilar_Marco/Materials/M_Color_Negro.M_Color_Negro"))