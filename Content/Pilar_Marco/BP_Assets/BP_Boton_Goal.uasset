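; Goal button actor that responds when the player character (BPC_Character_UMG) overlaps it.
; Its light sphere is black from the construction script, red at BeginPlay and green once the character overlaps.
; The overlap also calls UnlockTrapMessage on the referenced Trampa, then sets the mesh to single-node animation mode if the button's owner is a BP_Fairy_Guide.
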(event EventBeginPlay
  (Rendering|Material|SetMaterial (Variables|Default|GetEsfera_Luz) 0 "/Game/Pilar_Marco/Materials/M_Color_Rojo.M_Color_Rojo"))

(event Collision|EventActorBeginOverlap
  (params (OtherActor :type Actor%20Object%20Reference))
  (Utilities|Casting|CastToBPC_Character_UMG OtherActor)
  (Rendering|Material|SetMaterial (Variables|Default|GetEsfera_Luz) 0 "/Game/Pilar_Marco/Materials/M_Color_Verde.M_Color_Verde")
  (Class|BPIGame|UnlockTrap(Message) (Variables|Default|GetTrampa))
  (bind _asbp_fairy_guide (Utilities|Casting|CastToBP_Fairy_Guide (Components|GetOwner)))
  (Components|Animation|SetAnimationMode (Variables|/Script/Engine.Character|GetMesh _asbp_fairy_guide) "AnimationSingleNode" true))

(fn ConstructionScript
  (Rendering|Material|SetMaterial (Variables|Default|GetEsfera_Luz) 0 "/Game/Pilar_Marco/Materials/M_Color_Negro.M_Color_Negro"))